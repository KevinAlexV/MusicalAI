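; Player character Blueprint for a Paper2D flipbook character (Ben) in a 3D world, handling attacks, damage and animation.
; AttackA spawns a Swing actor and passes it Damage, while AttackB plays an attack flipbook and stops movement.
; The Attack event subtracts Health, launches the character away from the attacker and holds the hurt flipbook through a tick-counted cooldown.
; Tick otherwise picks idle, forward-run or back-run flipbooks from acceleration and camera distance versus boom length.
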(event Input|EnhancedActionEvents|EnhancedInputActionIA_AttackA
  (params (ActionValue :type Boolean) (ElapsedSeconds :type Float%20%28double-precision%29) (TriggeredSeconds :type Float%20%28double-precision%29) (InputAction :type Input%20Action%20Object%20Reference :default "/Game/MusicAI_GameMode/Input/Actions/IA_AttackA.IA_AttackA"))
  (bind _self self)
  (bind _playercharacter (Variables|Default|GetPlayerCharacter))
  (bind _returnvalue (Transformation|GetWorldTransform _playercharacter))
  (bind (_location _rotation) (Math|Transform|BreakTransform _returnvalue))
  (bind (_roll _pitch _yaw) (Math|Rotator|BreakRotator _rotation))
  (:Started
    (Development|PrintString "[BP_TPC] AttackA" false)
    (bind _returnvalue_2 (Game|SpawnActorfromClass "/Game/Characters/CharacterProps/Swing.Swing_C" (Math|Transform|MakeTransform (+ _location "") (Math|Rotator|MakeRotator _roll _pitch (+ _yaw 9e+01)) "1.000000,1.000000,1.000000") "AlwaysSpawn" _self _self))
    (Default|AttackAttempt _returnvalue_2 (Variables|Default|GetDamage))))

(event Input|EnhancedActionEvents|EnhancedInputActionIA_AttackB
  (params (ActionValue :type Boolean) (ElapsedSeconds :type Float%20%28double-precision%29) (TriggeredSeconds :type Float%20%28double-precision%29) (InputAction :type Input%20Action%20Object%20Reference :default "/Game/MusicAI_GameMode/Input/Actions/IA_AttackB.IA_AttackB"))
  (bind _playercharacter (Variables|Default|GetPlayerCharacter))
  (:Started
    (Sprite|SetFlipbook _playercharacter "/Game/Characters/SpriteSheets/Ben_AttackB.Ben_AttackB")
    (Audio|Components|Audio|Play _playercharacter)
    (Components|Movement|StopMovementImmediately (Variables|Character|GetCharacterMovement))))

(event Input|EnhancedActionEvents|EnhancedInputActionIA_Interact
  (params (ActionValue :type Boolean) (ElapsedSeconds :type Float%20%28double-precision%29) (TriggeredSeconds :type Float%20%28double-precision%29) (InputAction :type Input%20Action%20Object%20Reference :default "/Game/MusicAI_GameMode/Input/Actions/IA_Interact.IA_Interact"))
  (:Triggered
    (Development|PrintString "[BP_TPC] E" false false)))

(event EventTick
  (params (DeltaSeconds :type Float%20%28single-precision%29))
  (Variables|Default|SetMovingTowardsCam (>= (Variables|/Script/Engine.SpringArmComponent|GetTargetArmLength (Variables|Default|GetCameraBoom)) (Math|Vector|Distance(Vector) (Camera|GetCameraLocation (Game|GetPlayerCameraManager 0)) (Transformation|GetWorldLocation (Variables|Default|GetPlayerCharacter)))))
  (Utilities|FlowControl|Sequence
    (:then_0
      ;[1 1 1] Set velocity and ground speed from the movement components velocity. Ground speed is calculated from only the X and Y axis of the velocity, so moving up or down does not affect it.
      (bind _output_get (Variables|Default|SetVelocity (Variables|/Script/Engine.MovementComponent|GetVelocity (Variables|Character|GetCharacterMovement))))
      (Variables|Default|SetGroundSpeed (Math|Vector|VectorLengthXY _output_get)))
    (:then_1
      ;[1 1 1] Set Should Move to true only if ground speed is above a small threshold (to prevent incredibly small velocities from triggering animations) and if there is currently acceleration (input) applied.
      (Variables|Default|SetShouldMove (select (Pawn|IsPlayerControlled) (and (Utilities|Operators|NotEqual(!=) :A (Pawn|Components|CharacterMovement|GetCurrentAcceleration (Variables|Character|GetCharacterMovement))) (> (Variables|Default|GetGroundSpeed) 3.0)) (> (Variables|Default|GetGroundSpeed) 3.0)))
      (if (not (Variables|Default|GetIsCharging))
        (if (> (Variables|Default|GetAnimCooldown) 0.0)
          (Math|Float|DecrementFloat (Variables|Default|GetAnimCooldown))
          (else
            (if (Math|Vector|VectorIsZero (Pawn|Components|CharacterMovement|GetCurrentAcceleration (Variables|Character|GetCharacterMovement)))
              (Sprite|SetFlipbook (Variables|Default|GetPlayerCharacter) "/Game/Characters/SpriteSheets/Ben_Idle.Ben_Idle")
              (elif (Variables|Default|GetMovingTowardsCam)
                (Sprite|SetFlipbook (Variables|Default|GetPlayerCharacter) "/Game/Characters/SpriteSheets/Ben_RunForward.Ben_RunForward")
                (else
                  (Sprite|SetFlipbook (Variables|Default|GetPlayerCharacter) "/Game/Characters/SpriteSheets/Ben_RunBack.Ben_RunBack"))))
            (Audio|Components|Audio|Play (Variables|Default|GetPlayerCharacter))))))))

(event EventAttack
  (params (Damage :type Float%20%28double-precision%29) (Attacker :type Actor%20Object%20Reference))
  (bind _output_get (Variables|Default|SetHealth (- (Variables|Default|GetHealth) Damage)))
  (Sprite|SetFlipbook (Variables|Default|GetPlayerCharacter) "/Game/Characters/SpriteSheets/Ben_Hurt.Ben_Hurt")
  (Variables|Default|SetAnimCooldown 5.0)
  (bind _returnvalue (CallFunction|GetVectorBetweenObjects Attacker))
  (Character|LaunchCharacter (* _returnvalue 500) false false)
  (Development|PrintString "[BP_TPC] Hurt!" false true "(R=1.000000,G=0.000000,B=0.115187,A=1.000000)")
  (if (<= _output_get 0.0)
    (Development|PrintString "[BP_TPC] Game Over!" false true "(R=1.000000,G=0.000000,B=0.115187,A=1.000000)")))

(fn ConstructionScript)

(fn GetProjectileVector
  (bind _capsulecomponent (Variables|Default|GetCapsuleComponent))
  (bind _followcamera (Variables|Default|GetFollowCamera))
  (bind _returnvalue (Transformation|GetWorldLocation _followcamera))
  (bind _returnvalue_2 (Transformation|GetWorldLocation _capsulecomponent))
  (bind _returnvalue_3 (Math|Vector|GetUnitDirection(Vector) _returnvalue _returnvalue_2))
  (bind (_x _y) (Class|KismetMathLibrary|BreakVector3f _returnvalue_3))
  (bind _returnvalue_4 (Math|Vector|MakeVector _x _y 0.0))
  (Development|PrintString (Utilities|String|ToString(Vector) _returnvalue_4) false)
  (return _returnvalue_4))

(fn GetVectorBetweenObjects
  (params (Target :type Actor%20Object%20Reference))
  (bind _returnvalue (Transformation|GetActorLocation Target))
  (bind _capsulecomponent (Variables|Default|GetCapsuleComponent))
  (bind _returnvalue_2 (Transformation|GetWorldLocation _capsulecomponent))
  (bind _returnvalue_3 (Math|Vector|GetUnitDirection(Vector) _returnvalue _returnvalue_2))
  (bind (_x _y) (Class|KismetMathLibrary|BreakVector3f _returnvalue_3))
  (Utilities|IsValid Target
    (:Is%20Valid
      (return (Math|Vector|MakeVector _x _y 0.0)))
    (:Is%20Not%20Valid
      (return "0, 0, 0"))))